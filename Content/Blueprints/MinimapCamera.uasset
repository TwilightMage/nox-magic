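; Minimap camera actor that follows the player and renders the map view through its MinimapCapture scene capture component.
; On BeginPlay it hides the components of all existing Character and Drop actors from the capture.
; Each tick it teleports to the location of the Player reference when that is valid, changing only position.
; The Ignoreactor event lets other code hide additional actors from the capture at runtime.
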(event Custom|Ignore%20actor
  (params (actor :type Actor%20Object%20Reference))
  (Class|SceneCaptureComponent|HideActorComponents (Variables|Default|GetMinimapCapture) actor))

(event EventBeginPlay
  (bind _minimapcapture (Variables|Default|GetMinimapCapture))
  (Utilities|FlowControl|Sequence
    (:then_0
      (bind _outactors (Actor|GetAllActorsOfClass "/Script/Engine.Character"))
      (for _array_element _outactors
        (Class|SceneCaptureComponent|HideActorComponents _minimapcapture _array_element)))
    (:then_1
      (bind _outactors_2 (Actor|GetAllActorsOfClass "/Game/Blueprints/Drop.Drop_C"))
      (for _array_element_2 _outactors_2
        (Class|SceneCaptureComponent|HideActorComponents _minimapcapture _array_element_2)))))

(event EventTick
  (params (DeltaSeconds :type Float%20%28single-precision%29))
  (bind _player (Variables|Default|Getplayer))
  (Utilities|IsValid _player
    (:Is%20Valid
      (Transformation|SetActorLocation (Transformation|GetActorLocation _player) false true))))

(fn ConstructionScript)