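; Spell object that runs a cast from its Data and produces a spell actor through its Caster.
; Cast time scales with the number of Data nodes and counts down on Tick, while Stopcast flags an interruption; both outcomes fire the Stoped dispatcher.
; On completion, the spawned actor gets its skeletal mesh from the shape, material from the element, and target of either none or the caster.
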(event Custom|Stop%20cast
  (Variables|Default|Setinterupted true))

(event Custom|Begin%20cast
  (Variables|cast|Settime%20casted (CallFunction|CastTime)))

(event Custom|Copy%20from
  (params (target :type Spell%20Object%20Reference))
  (Variables|Default|Setdata (Variables|Spell_C|Getdata target)))

(event Custom|Tick
  (params (delta%20time :type Float%20%28single-precision%29))
  (if (Variables|Default|Getinterupted)
    (Default|CallStoped "NewEnumerator0")
    (else
      (bind _output_get (Variables|cast|Settime%20casted (- (Variables|cast|Gettime%20casted) delta%20time)))
      (if (<= _output_get 0.0)
        (bind _actor (Default|SpawnSpellActor (Variables|Default|Getcaster) (Variables|Default|Getdata)))
        (Utilities|FlowControl|Sequence
          (:then_0
            (|Setupmesh (Variables|/Game/Blueprints/SpellActor.SpellActor_C|GetSkeletalMesh _actor)))
          (:then_1
            (|Setupmaterial (Variables|/Game/Blueprints/SpellActor.SpellActor_C|GetSkeletalMesh _actor)))
          (:then_2
            (|Setuptarget _actor))
          (:then_3
            (Default|CallStoped "NewEnumerator2")))))))

(fn CastTime
  (return (* (Utilities|Array|Length (.nodes (Utilities|Struct|BreakSpellData (Variables|Default|Getdata)))) 0.123)))