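; NoxMagic function library that builds spells from rune node trees and provides shared item, text and UI helpers.
; ConstructSpell matches each top-level branch against element, shape, target and existence pattern assets, filling SpellData, with DefinedTrees blocking repeat matches.
; Other helpers fetch item defaults from type-specific data tables, look up shape and element data in NM_Container, match wildcard word sequences and open confirm boxes.
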(fn FetchDefaults
  (params (name :type Name))
  (bind _returnvalue (Class|DataTableFunctionLibrary|DoesDataTableRowExist "/Game/Datatables/Items/ItemDefaults.ItemDefaults" name))
  (bind _returnvalue_2 (Utilities|GetDataTableRow "/Game/Datatables/Items/ItemDefaults.ItemDefaults" (select _returnvalue name "Undefined"))
    (:then
      (switch Utilities|FlowControl|Switch|SwitchonItemType (.itemtype (Utilities|Struct|BreakItemDefault _returnvalue_2))
        (:NewEnumerator2
          (return true _returnvalue_2 "" "" "" ""))
        (:NewEnumerator0
          (bind _returnvalue_3 (Utilities|GetDataTableRow "/Game/Datatables/Items/MeleeWeaponDefaults.MeleeWeaponDefaults" name)
            (:then
              (return true _returnvalue_2 _returnvalue_3 "" "" ""))
            (:RowNotFound
              _)))
        (:NewEnumerator1
          (bind _returnvalue_4 (Utilities|GetDataTableRow "/Game/Datatables/Items/StaffDefaults.StaffDefaults" name)
            (:then
              (return true "" "" _returnvalue_4 "" ""))
            (:RowNotFound
              _)))
        (:NewEnumerator3
          (bind _returnvalue_5 (Utilities|GetDataTableRow "/Game/Datatables/Items/BowDefaults.BowDefaults" name)
            (:then
              (return true "" "" "" _returnvalue_5 ""))
            (:RowNotFound
              _)))
        (:NewEnumerator4
          (bind _returnvalue_6 (Utilities|GetDataTableRow "/Game/Datatables/Items/ArmorDefaults.ArmorDefaults" name :!label _label)
            (:then
              (return true "" "" "" "" _returnvalue_6))
            (:RowNotFound
              _)))
        (:NewEnumerator5
          (goto _label))
        (:NewEnumerator6
          (goto _label))
        (:NewEnumerator7
          (goto _label))
        (:NewEnumerator8
          (goto _label))
        (:NewEnumerator9
          (goto _label))))
    (:RowNotFound
      _))
  (return false "" "" "" "" ""))

(fn MakeItemCodeValid
  (params (in :type Name))
  (bind _returnvalue (Class|DataTableFunctionLibrary|DoesDataTableRowExist "/Game/Datatables/Items/ItemDefaults.ItemDefaults" in))
  (return (select (and _returnvalue (Utilities|Name|NotEqual(Name) in "None")) in "Undefined")))

(fn ConstructSpell
  (params (nodes :type Array%20of%20Tree%20Node%20Structures) (parents :type Map%20of%20Integers%20to%20Integers) (outer :type Object%20Object%20Reference))
  (bind _defined_trees (LocalVariables|Getdefined%20trees))
  (Utilities|Struct|SetmembersinSpellData (LocalVariables|Getresult%20data) nodes parents)
  (bind _returnvalue (Game|ConstructObjectfromClass "/Game/Blueprints/Spell.Spell_C" outer))
  (bind _output_get (LocalVariables|Setresult _returnvalue))
  (for _array_element (Variables|/Script/NoxMagic.TreeNodeDynamic|Getchildren (Class|TreeAsset|FormTree nodes parents))
    (|SetupElement _array_element _defined_trees
      (:Fail
        (|Setupshape _array_element _defined_trees
          (:Fail
            (|Setuptarget _array_element _defined_trees
              (:Fail
                (|Setupexistance _array_element _defined_trees
                  (:Fail
                    (return 0))))))))))
  (Variables|/Game/Blueprints/Spell.Spell_C|Setdata _output_get (LocalVariables|Getresult%20data))
  (return _output_get))

(fn FetchWordCombination
  (params (words :type String) (combination :type String))
  (bind _returnvalue (Class|NoxMagicFunctions|StringtoArray combination))
  (bind _marked_words_buffer (LocalVariables|Getmarked%20words%20buffer))
  (for _array_element (Class|NoxMagicFunctions|StringtoArray words)
    (if (Utilities|Enum|Equal(Enum) _array_element (Utilities|Array|Get(acopy) _returnvalue (LocalVariables|Getcombination%20position))) :!label _label
      (Math|Integer|IncrementInt (LocalVariables|Getcombination%20position)
        (:%20%20
          (bind _output_get (LocalVariables|Setfull (Utilities|String|Append (LocalVariables|Getfull) " " _array_element) :!label _label_2))
          (if (== (LocalVariables|Getcombination%20position) (Utilities|Array|Length _returnvalue))
            (return _marked_words_buffer true (Utilities|String|Trim _output_get)))))
      (elif (Utilities|Enum|Equal(Enum) (Utilities|Array|Get(acopy) _returnvalue (LocalVariables|Getcombination%20position)) "*")
        (Math|Integer|IncrementInt (LocalVariables|Getcombination%20position)
          (:%20%20
            (Utilities|Array|Add _marked_words_buffer _array_element)
            (goto _label_2)))
        (elif (> (LocalVariables|Getcombination%20position) 0)
          (LocalVariables|Setcombination%20position 0)
          (Utilities|Array|Clear _marked_words_buffer)
          (LocalVariables|Setfull "")
          (goto _label)
          (else
            (Utilities|Array|Clear _marked_words_buffer)
            (LocalVariables|Setfull ""))))))
  (return 0 false ""))

(fn GetAllObjectTypes
  (bind _result (LocalVariables|Getresult))
  (for _index (range 0 (- (|GetNumEnumEntries) 1))
    (Utilities|Array|Add _result (Utilities|Enum|ByteToEnumEObjectTypeQuery (Math|Conversions|ToByte(Integer) _index))))
  (return _result))

(fn FetchSpellShapeData
  (params (shape :type Spell_Shape%20Enum :default "NewEnumerator0"))
  (bind _returnvalue (Class|DataContainer|GetContainer "/Game/Blueprints/GameClasses/NoxMagic/NM_Container.NM_Container_C")
    (:Success
      (return (.Value (Utilities|Map|Find (Variables|/Game/Blueprints/GameClasses/NoxMagic/NM_Container.NM_Container_C|Getspell%20shape%20data _returnvalue) shape))))))

(fn FetchSpellElementData
  (params (element :type Spell_Element%20Enum :default "NewEnumerator0"))
  (bind _returnvalue (Class|DataContainer|GetContainer "/Game/Blueprints/GameClasses/NoxMagic/NM_Container.NM_Container_C")
    (:Success
      (return (.Value (Utilities|Map|Find (Variables|/Game/Blueprints/GameClasses/NoxMagic/NM_Container.NM_Container_C|Getspell%20element%20data _returnvalue) element))))))

(fn Ask
  (params (TItle :type Text) (Content :type Text) (Yes :type Text) (No :type Text) (on%20No :type Delegate%20%28by%20ref%29) (On%20Yes :type Delegate%20%28by%20ref%29))
  (bind _returnvalue (UserInterface|CreateWidget "/Game/UI/ConfirmBox.ConfirmBox_C" 0 TItle Content Yes No))
  (EventDispatchers|BindEventtoChooseNo _returnvalue on%20No)
  (EventDispatchers|BindEventtoChooseYes _returnvalue On%20Yes)
  (UserInterface|Viewport|AddtoPlayerScreen _returnvalue))

(fn MatchTreesAdvanced
  (params (source :type Tree%20Node%20Dynamic%20Object%20Reference) (asset :type Tree%20Asset%20Object%20Reference) (defined%20trees :type Array%20of%20Strings))
  (bind _returnvalue (Utilities|GetObjectName asset))
  (bind _returnvalue_2 (Class|TreeAsset|FormTreefromAsset asset))
  (bind (_matchedtrees _matchedrunes _success) (Class|TreeNodeDynamic|MatchTrees source _returnvalue_2))
  (if (and _success (not (Utilities|Array|ContainsItem defined%20trees _returnvalue)))
    (Utilities|Array|Add defined%20trees _returnvalue)
    (return _matchedtrees _matchedrunes true)
    (else
      (return 0 0 false))))

(fn SearchTree
  (params (tree :type Tree%20Node%20Dynamic%20Object%20Reference) (variants :type Array%20of%20Tree%20Asset%20Object%20References) (defined%20trees :type Array%20of%20Strings))
  (for _array_element variants
    (if (and (.success (Class|TreeNodeDynamic|MatchTrees tree (Class|TreeAsset|FormTreefromAsset _array_element))) (not (Utilities|Array|ContainsItem defined%20trees (Utilities|GetObjectName _array_element))))
      (Utilities|Array|Add defined%20trees (Utilities|GetObjectName _array_element))
      (return _array_element true (.matchedTrees (Class|TreeNodeDynamic|MatchTrees tree (Class|TreeAsset|FormTreefromAsset _array_element))) (.matchedRunes (Class|TreeNodeDynamic|MatchTrees tree (Class|TreeAsset|FormTreefromAsset _array_element))))))
  (return 0 false 0 0))