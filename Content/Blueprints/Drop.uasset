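; Dropped item actor that players highlight and pick up through its Interactive component, which passes it to the player's inventory server call.
; On BeginPlay it fetches item defaults by content ID, while its construction script sets the mesh and enables physics if the ID has a data table row.
; Disappearing sets a short lifespan and plays a colored, bounds-scaled particle burst with a timeline-driven dissolve on clients.
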(event OnInteraction(Interactive)
  (params (player :type ALS%20Base%20Character%20Object%20Reference))
  (|DoInteraction player))

(event OnHightlight(Interactive)
  (params (state :type Boolean))
  (|DoOnHightlight state))

(event Custom|Load%20content%20from%20database
  (bind (_success _default _melee_weapon_default _staff_default _bow_default _armor_default) (CallFunction|FetchDefaults (Utilities|Struct|BreakItem (Variables|Default|Getcontent))))
  (Variables|Default|Setcontent (Utilities|Struct|MakeItem (Utilities|Struct|BreakItem (Variables|Default|Getcontent)) _default _melee_weapon_default _staff_default _bow_default _armor_default)))

(event Custom|Disapear
  (params (color :type Linear%20Color%20Structure))
  ;[1 1 1] Disapear
  (CallFunction|DisapearonClients color)
  (Actor|SetLifeSpan 5.0) ; Wait before initialising disapear\neffect on all clients
)

(event Custom|Disapear%20on%20clients
  (params (color :type Linear%20Color%20Structure))
  ;[1 1 1] Disapear
  (|Dodisapear color))

(event EventBeginPlay
  (bind _content (Variables|Default|Getcontent))
  (bind (_id _default) (Utilities|Struct|BreakItem _content))
  (if (Utilities|Name|NotEqual(Name) _id "None")
    (CallFunction|LoadContentfromDatabase))
  (Variables|/Game/Blueprints/Interactive.Interactive_C|Setdisplay%20name (Variables|Default|GetInteractive) (Utilities|Struct|BreakItemDefault _default)))

(event Collision|EventActorBeginOverlap
  (params (OtherActor :type Actor%20Object%20Reference)))

(fn ConstructionScript
  (bind _content (Variables|Default|Getcontent))
  (bind _skeletalmesh (Variables|Default|GetSkeletalMesh))
  (bind (_id _default) (Utilities|Struct|BreakItem _content))
  (bind _mesh (Utilities|Struct|BreakItemDefault _default))
  (bind _out (CallFunction|MakeItemCodeValid _id))
  (bind _returnvalue (Utilities|GetDataTableRow "/Game/Datatables/Items/ItemDefaults.ItemDefaults" _out)
    (:then
      (Class|SkinnedMeshComponent|SetSkeletalMesh _skeletalmesh (select (!= _mesh 0) _mesh (Utilities|Struct|BreakItemDefault _returnvalue)) true)
      (Physics|SetSimulatePhysics _skeletalmesh true))
    (:RowNotFound
      (Class|SkinnedMeshComponent|SetSkeletalMesh _skeletalmesh 0 true)
      (Physics|SetSimulatePhysics _skeletalmesh false))))