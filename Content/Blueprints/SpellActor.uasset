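; Spell actor defined by element and shape data, which set its display name, speed modifier and light color; per-shape branches are still empty.
; Each tick it can follow its target using distance-based speed curves, with Followable targets supplying the follow transform.
; It drains caster mana continuously and destroys itself when draining fails, a fixed lifetime expires or its caster interacts with it.
; Interaction highlighting uses custom depth.
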(event OnInteraction(Interactive)
  (params (player :type ALS%20Base%20Character%20Object%20Reference))
  (|Dooninteraction player))

(event OnHightlight(Interactive)
  (params (state :type Boolean))
  (|Doonhighlight state))

(event Custom|Dispose
  (Actor|DestroyActor))

(event EventBeginPlay
  (Utilities|FlowControl|Sequence
    (:then_0
      (|Fetchdata))
    (:then_1
      (|Setuplifetime))
    (:then_2
      (|Processshape))
    (:then_3
      (|Setupdisplayname))))

(event EventTick
  (params (DeltaSeconds :type Float%20%28single-precision%29))
  (Utilities|FlowControl|Sequence
    (:then_0
      (|Spendlifetime))
    (:then_1
      (|Follow))
    (:then_2
      (|Drainmana))))

(fn ConstructionScript)