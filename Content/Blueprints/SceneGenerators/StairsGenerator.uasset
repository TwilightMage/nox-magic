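; StairsGenerator is a Blueprint that procedurally builds a staircase from a configurable mesh.
; Its Construction Script clears and refills an InstancedStaticMesh component through nested loops over horizontal and vertical counts.
; Columns spread symmetrically along Y by the mesh's bounding width, giving twice HorizontalCount minus one per step.
; Steps advance along X by ForwardOffset and rise or descend by mesh height according to ExpandUp.
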(event EventBeginPlay)

(event Collision|EventActorBeginOverlap
  (params (OtherActor :type Actor%20Object%20Reference)))

(event EventTick
  (params (DeltaSeconds :type Float%20%28single-precision%29)))

(fn ConstructionScript
  (bind _horizontal_count (Variables|Default|Gethorizontal%20count))
  (bind _mesh (Variables|Default|Getmesh))
  (bind _instancedstaticmesh (Variables|Default|GetInstancedStaticMesh))
  (bind _returnvalue (- _horizontal_count 1))
  (bind _returnvalue_2 (StaticMesh|GetBoundingBox _mesh))
  (bind (_min _max) (Utilities|Struct|BreakBox _returnvalue_2))
  (bind _returnvalue_3 (- _max _min))
  (bind (_x _y _z) (Math|Vector|BreakVector _returnvalue_3))
  (Components|StaticMesh|SetStaticMesh _instancedstaticmesh (Variables|Default|Getmesh))
  (Components|InstancedStaticMesh|ClearInstances _instancedstaticmesh)
  (for _index (range (* _returnvalue -1) _returnvalue)
    (for _index_2 (range 0 (- (Variables|Default|Getvertical%20count) 1))
      (Components|InstancedStaticMesh|AddInstance (Variables|Default|GetInstancedStaticMesh) (Math|Transform|MakeTransform (Math|Vector|MakeVector (* (Variables|Default|Getforward%20offset) (Math|Conversions|ToFloat(Integer) _index_2)) (+ (* _index _y) 1.0) (* (* _index_2 _z) (select (Variables|Default|Getexpand%20up) 1.0 -1.0))) (Variables|Default|Getrotation))))))