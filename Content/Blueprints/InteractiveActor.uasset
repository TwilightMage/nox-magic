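; InteractiveActor is an interactable mesh actor that binds its interaction and highlight handlers to an Interactive component on BeginPlay.
; Highlighting toggles the mesh's custom depth rendering, while the interaction handler is empty.
; A SyncPlv event applies a given linear velocity and teleports the mesh to a given transform.
; The server-side velocity-change check that would call SyncPlv is disconnected and never runs.
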(event Custom|On%20interaction
  (params (player :type ALS%20Base%20Character%20Object%20Reference)))

(event Custom|On%20Hightlight
  (params (state :type Boolean))
  (Rendering|SetRenderCustomDepth (Variables|Default|GetMesh) state))

(event Custom|Sync%20plv
  (params (plv :type Vector) (location :type Vector) (rotation :type Rotator))
  (bind _mesh (Variables|Default|GetMesh))
  (Physics|SetPhysicsLinearVelocity _mesh plv false "None")
  (Transformation|SetWorldLocationAndRotation _mesh location rotation false true))

(event EventBeginPlay
  (|Assignevents (delegate Custom|On%20interaction) (delegate Custom|On%20Hightlight)))

(event Collision|EventActorBeginOverlap
  (params (OtherActor :type Actor%20Object%20Reference)))

(event EventTick
  (params (DeltaSeconds :type Float%20%28single-precision%29)))

(fn ConstructionScript)